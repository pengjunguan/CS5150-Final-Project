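; Scout variant of the AI character that handles its own damage and death.
; While alive, it subtracts incoming damage from Health, printing the value before and after.
; At zero health, if its controller has a valid Blackboard, it sets the BNeedShareTarget key true, marks itself dead and calls AIDeath.
; Without a valid Blackboard the death step is skipped; construction only runs the parent script.
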(event EventBeginPlay
  (|CallParentFunction) ; This node is disabled and will not be called.\nDrag off pins to build functionality.
)

(event Collision|EventActorBeginOverlap
  (params (OtherActor :type Actor%20Object%20Reference))
  (|CallParentFunction OtherActor) ; This node is disabled and will not be called.\nDrag off pins to build functionality.
)

(event EventTick
  (params (DeltaSeconds :type Float%20%28single-precision%29))
  (|CallParentFunction DeltaSeconds) ; This node is disabled and will not be called.\nDrag off pins to build functionality.
)

(event Game|Damage|EventAnyDamage
  (params (Damage :type Float%20%28single-precision%29) (DamageType :type Damage%20Type%20Object%20Reference) (InstigatedBy :type Controller%20Object%20Reference) (DamageCauser :type Actor%20Object%20Reference))
  (bind _returnvalue (Pawn|GetController))
  (bind _returnvalue_2 (AI|GetBlackboard _returnvalue))
  (if (not (Variables|Default|GetbIsDead))
    (Development|PrintString (Utilities|String|Append (Utilities|String|ToString(Float) (Variables|Default|GetHealth)) "Health"))
    (bind _output_get (Variables|Default|SetHealth (- (Variables|Default|GetHealth) Damage)))
    (Development|PrintString (Utilities|String|Append (Utilities|String|ToString(Float) _output_get) "Health"))
    (if (<= (Variables|Default|GetHealth) 0.0)
      (if (not (Variables|Default|GetbIsDead))
        (Utilities|IsValid _returnvalue_2
          (:Is%20Valid
            (AI|Components|Blackboard|SetValueasBool _returnvalue_2 (Variables|Default|Getb%20Need%20Share%20Target) true)
            (Variables|Default|SetbIsDead true)
            (CallFunction|AIDeath)))))))

(fn ConstructionScript
  (|CallParentFunction))