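; Base enemy AI Blueprint that provides query functions for health, target range and retreat decisions, with an empty event graph.
; Attack and sight checks validate the target, then compare its distance to AttackRange or SightRange; sight has no line-of-sight trace.
; GetHealthRatio only returns a same-named call's result.
; ShouldRetreat is a stub that always returns false, leaving LowHealthThreshold unused, and GetPlayerCharacterRef is empty.
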(event EventBeginPlay)

(event Collision|EventActorBeginOverlap
  (params (OtherActor :type Actor%20Object%20Reference)))

(event EventTick
  (params (DeltaSeconds :type Float%20%28single-precision%29)))

(fn ConstructionScript)

(fn GetPlayerCharacterRef)

(fn GetHealthRatio
  (bind _healthratio (CallFunction|GetHealthRatio))
  (return _healthratio))

(fn IsTargetinAttackRange
  (params (TargetActor :type Actor%20Object%20Reference))
  (Utilities|IsValid TargetActor
    (:Is%20Valid
      (return (<= (Math|Vector|Distance(Vector) (Transformation|GetActorLocation TargetActor) (Transformation|GetActorLocation)) (Variables|Default|GetAttackRange))))
    (:Is%20Not%20Valid
      (Development|PrintString "IsTargetInAttackRange: Get Target Actor Failed."))))

(fn CanSeeTarget
  (params (TargetActor :type Actor%20Object%20Reference))
  (Utilities|IsValid TargetActor
    (:Is%20Valid
      (return (<= (Math|Vector|Distance(Vector) (Transformation|GetActorLocation TargetActor) (Transformation|GetActorLocation)) (Variables|Default|GetSightRange))))
    (:Is%20Not%20Valid
      (Development|PrintString "CanSeeTarget: Get Target Actor Failed."))))

(fn ShouldRetreat
  (CallFunction|GetHealthRatio)
  (return false))