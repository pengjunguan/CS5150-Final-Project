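; BP_VitalityComponent is a health component in the EnemyAI folder that stores HP and death state.
; Kill zeroes HP and runs ExecuteDeath, which sets IsDead and fires the Death dispatcher.
; Helpers return the HP-to-MaxHP ratio and add healing without clamping.
; IsLowHealth is unfinished: it ignores its threshold and always returns false, and no damage handling exists here.
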(event Custom|ExecuteDeath
  (Variables|Default|SetIsDead true)
  (Default|CallDeath))

(event Custom|Kill
  (Variables|Default|SetHP 0.0)
  (CallFunction|ExecuteDeath))

(event EventBeginPlay)

(event EventTick
  (params (DeltaSeconds :type Float%20%28single-precision%29)))

(fn GetHealthRatio
  (return (/ (Variables|Default|GetHP) (Variables|Default|GetMaxHP))))

(fn IsLowHealth
  (params (Threshold :type Float%20%28double-precision%29))
  (CallFunction|GetHealthRatio)
  (return false))

(fn Heal
  (params (Amount :type Float%20%28double-precision%29))
  (Variables|Default|SetHP (+ Amount (Variables|Default|GetHP))))